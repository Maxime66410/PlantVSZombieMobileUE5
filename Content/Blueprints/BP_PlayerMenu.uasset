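; BP_PlayerMenu is a player controller that sets up mobile input and chooses the opening menu screen on BeginPlay.
; It adds the IMC_MobileDefault mapping context, then checks the inventory in the custom game instance's save.
; An empty inventory shows the first-invocation widget, while a filled one creates and stores the main menu widget.
; Both steps run only when the Enhanced Input subsystem is valid.
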(event EventBeginPlay
  (bind _returnvalue (PlayerController|LocalPlayerSubsystems|GetEnhancedInputLocalPlayerSubsystem))
  (Utilities|IsValid _returnvalue
    (:Is%20Valid
      (Input|AddMappingContext _returnvalue "/Game/Input/IMC_MobileDefault.IMC_MobileDefault" 0 "(bIgnoreAllPressedKeysUntilRelease=True,bForceImmediately=False,bNotifyUserSettings=False)")
      (if (Utilities|Array|IsEmpty (Variables|/Game/Blueprints/Save/BP_SaveCustom.BP_SaveCustom_C|GetInventaire (Variables|/Game/Blueprints/BP_CustomGameInstance.BP_CustomGameInstance_C|GetSaveRef (.AsBP%20Custom%20Game%20Instance (Utilities|Casting|CastToBP_CustomGameInstance (Game|GetGameInstance))))))
        (bind _returnvalue_2 (UserInterface|CreateWidget "/Game/Widget/Gacha/WBP_InvocationFirst.WBP_InvocationFirst_C"))
        (UserInterface|Viewport|AddtoViewport _returnvalue_2 0)
        (else
          (bind _returnvalue_3 (UserInterface|CreateWidget "/Game/Blueprints/UI/UW_MainMenu.UW_MainMenu_C" self))
          (bind _output_get (Variables|Default|SetMainMenu _returnvalue_3))
          (UserInterface|Viewport|AddtoViewport _output_get 0))))))

(fn ConstructionScript)