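; Dungeon manager actor that swings open a door at the start of play and creates dragon egg meshes, apparently as reward spawners.
; One second after BeginPlay, OpenDoor plays two timelines that lerp the yaw of two arrow components 80 degrees in opposite directions.
; The construction script adds one manually attached dragon egg skeletal mesh per NmbSpawnerReward, each placed with a GetRelativeTransform result.
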(event Custom|Open%20Door
  (Utilities|FlowControl|Sequence
    (:then_0
      (bind _rotate (Timeline|Door Play)
        (:Update
          (Transformation|SetRelativeRotation (Variables|Default|GetArrowP) (Math|Rotator|MakeRotator 0.0 0.0 (Math|Float|Lerp 0.0 8e+01 _rotate)) false false))))
    (:then_1
      (bind _rotate_2 (Timeline|Timeline Play)
        (:Update
          (Transformation|SetRelativeRotation (Variables|Default|GetArrowN) (Math|Rotator|MakeRotator 0.0 0.0 (Math|Float|Lerp 0.0 -8e+01 _rotate_2)) false false))))))

(event EventBeginPlay
  (Utilities|FlowControl|Delay 1.0)
  (CallFunction|OpenDoor))

(fn ConstructionScript
  (for _index (range 0 (- (Variables|Default|GetNmbSpawnerReward) 1))
    (bind _returnvalue (AddComponent|AddSkeletalMeshComponent true (Transformation|GetRelativeTransform)))
    (bind _output_get (Variables|Default|SetSkEgg _returnvalue))
    (Components|SkeletalMesh|SetSkeletalMeshAsset _output_get "/Game/LittleDragons/Meshes/SK_Dragon_Egg.SK_Dragon_Egg")))