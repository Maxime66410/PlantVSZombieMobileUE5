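; Player controller for grid-based unit placement with mobile input, spawning a BP_PlantSimple on the touched tile.
; BeginPlay shows the cursor, adds the mobile mapping context and, after a temporary delay, finds BP_Grid and creates the WBP_MorganDeck widget.
; IA_Touch converts the under-cursor hit to a tile and spawns the plant at its center at fixed height; its line trace result is unused.
; Finger-tracked dragon placement with tile highlighting remains as disconnected logic.
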(event Input|EnhancedActionEvents|EnhancedInputActionIA_Touch
  (params (ActionValue :type Boolean) (ElapsedSeconds :type Float%20%28double-precision%29) (TriggeredSeconds :type Float%20%28double-precision%29) (InputAction :type Input%20Action%20Object%20Reference :default "/Game/Input/Action/IA_Touch.IA_Touch")))

(event Input|EnhancedActionEvents|EnhancedInputActionIA_Touch
  (params (ActionValue :type Boolean) (ElapsedSeconds :type Float%20%28double-precision%29) (TriggeredSeconds :type Float%20%28double-precision%29) (InputAction :type Input%20Action%20Object%20Reference :default "/Game/Input/Action/IA_Touch.IA_Touch"))
  (bind _gridref (Variables|Default|GetGridRef))
  (:Started
    (bind (_valid_ _row _column) (Default|LocationtoTile _gridref (.Location (Collision|BreakHitResult (.HitResult (Game|Player|GetHitResultUnderCursorbyChannel "TraceTypeQuery1" true))))))
    (if _valid_
      (bind _gridlocation (Default|TiletoGridLocation _gridref _row _column true))
      (bind _outhit (Collision|LineTraceByChannel (Math|Conversions|ToVector(Vector2D) _gridlocation 3.1e+02) (Math|Conversions|ToVector(Vector2D) _gridlocation 3.1e+02) "TraceTypeQuery1" false 0 "None"))
      (bind _returnvalue (Game|SpawnActorfromClass :Class "/Game/Blueprints/Plants/BP_PlantSimple.BP_PlantSimple_C" :SpawnTransform (Math|Transform|MakeTransform (Math|Conversions|ToVector(Vector2D) _gridlocation 3.1e+02) "0, 0, 0" "1.000000,1.000000,1.000000") :CollisionHandlingOverride "Undefined" :TransformScaleMethod "MultiplyWithRoot" :Instigator 0))
      (Development|PrintString (Utilities|String|ToString(Vector) (Transformation|GetActorLocation _returnvalue)) true true "(R=0.000000,G=1.000000,B=0.083652,A=1.000000)"))))

(event EventBeginPlay
  (bind _returnvalue (PlayerController|LocalPlayerSubsystems|GetEnhancedInputLocalPlayerSubsystem))
  (Variables|/Script/Engine.PlayerController|SetbShowMouseCursor (Game|GetPlayerController 0) true)
  (Utilities|IsValid _returnvalue
    (:Is%20Valid
      (Input|AddMappingContext _returnvalue "/Game/Input/IMC_MobileDefault.IMC_MobileDefault" 0 "(bIgnoreAllPressedKeysUntilRelease=True,bForceImmediately=False,bNotifyUserSettings=False)")
      ;[1 0 0] TEMPORAIRE
      (Utilities|FlowControl|Delay 1.0)
      (bind _returnvalue_2 (Actor|GetActorOfClass "/Game/Blueprints/BP_Grid.BP_Grid_C"))
      (bind _output_get (Variables|Default|SetGridRef _returnvalue_2))
      (bind _returnvalue_3 (UserInterface|CreateWidget "/Game/Widget/DragAndDropCards/WBP_MorganDeck.WBP_MorganDeck_C" 0 _output_get self))
      (UserInterface|Viewport|AddtoViewport _returnvalue_3 0))))

(fn ConstructionScript)