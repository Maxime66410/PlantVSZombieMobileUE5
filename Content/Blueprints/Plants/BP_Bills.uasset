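; BP_Bills is a plant that periodically spawns a sun pickup (BP_Soleil) at its own location.
; On BeginPlay it starts a looping timer with a random interval, picked once per instance.
; Each spawn plays a timeline that moves the new sun along a random horizontal direction with a fixed upward component, scaled by the timeline track on every update.
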(event Custom|SpawnSun
  (bind _returnvalue (Math|Random|RandomUnitVector))
  (bind _returnvalue_2 (Game|SpawnActorfromClass "/Game/Blueprints/Soleil/BP_Soleil.BP_Soleil_C" (Math|Transform|MakeTransform (.location (Transformation|GetActorTransform)) "0, 0, 0" "1.000000,1.000000,1.000000") "AlwaysSpawn" "MultiplyWithRoot" 0 0))
  (Variables|Default|SetNewVar (Math|Vector|MakeVector (.x _returnvalue) (.y _returnvalue) 0.3))
  (bind _newtrack_0 (Timeline|Timeline PlayFromStart)
    (:Update
      (Transformation|SetActorLocation _returnvalue_2 (+ (Transformation|GetActorLocation _returnvalue_2) (* (Variables|Default|GetNewVar) _newtrack_0 2.0)) false false))))

(event EventBeginPlay
  (|CallParentFunction)
  (Utilities|Time|SetTimerbyEvent (delegate Custom|SpawnSun) (Math|Random|RandomFloatinRange 7.0 2e+01) true))

(event Collision|EventActorBeginOverlap
  (params (OtherActor :type Actor%20Object%20Reference)))

(event EventTick
  (params (DeltaSeconds :type Float%20%28single-precision%29))
  (|CallParentFunction DeltaSeconds) ; This node is disabled and will not be called.\nDrag off pins to build functionality.
)

(fn ConstructionScript
  (|CallParentFunction))