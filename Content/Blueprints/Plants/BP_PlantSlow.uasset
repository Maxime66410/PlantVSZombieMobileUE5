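; Child plant Blueprint, named as a slow-type plant, that raises an attack flag on a repeating timer; no slowing effect is defined here.
; BeginPlay runs the parent logic, then starts a looping timer at the plant stats' ShootRate.
; Shoot sets IsAttack if not already set; nothing in this graph clears it.
; RefreshAttackSpeed clears and recreates the timer so it uses the current ShootRate.
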(event EventBeginPlay
  (|CallParentFunction)
  (bind _returnvalue (Utilities|Time|SetTimerbyEvent (delegate EventShoot) (.shootrate (Variables|Default|GetStatsPlante)) true))
  (Variables|Default|SetEvent_Attack _returnvalue))

(event Collision|EventActorBeginOverlap
  (params (OtherActor :type Actor%20Object%20Reference))
  (|CallParentFunction OtherActor) ; This node is disabled and will not be called.\nDrag off pins to build functionality.
)

(event EventTick
  (params (DeltaSeconds :type Float%20%28single-precision%29))
  (|CallParentFunction DeltaSeconds) ; This node is disabled and will not be called.\nDrag off pins to build functionality.
)

(event EventShoot
  (if (not (Variables|Default|GetIsAttack))
    (Variables|Default|SetIsAttack true)))

(event EventRefreshAttackSpeed
  (Utilities|Time|ClearandInvalidateTimerbyHandle (Variables|Default|GetEvent_Attack))
  (bind _returnvalue (Utilities|Time|SetTimerbyEvent (EventDispatchers|CreateEvent :!event Shoot) (.shootrate (Variables|Default|GetStatsPlante)) true))
  (Variables|Default|SetEvent_Attack _returnvalue))

(fn ConstructionScript
  (|CallParentFunction))