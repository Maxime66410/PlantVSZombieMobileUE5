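; BP_PlantTrap is a plant trap that briefly stuns a zombie that enters its box, then removes itself.
; Box overlap with a BP_ZombieParent plays an attack montage, whose notify disables the zombie's movement and sets both stun flags.
; When the montage completes, a timeline sinks the mesh, then restores the zombie and destroys the trap.
; The trap's IsStun flag blocks new overlaps only from the notify onward.
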(event OnComponentBeginOverlap(Box)
  (params (OverlappedComponent :type Primitive%20Component%20Object%20Reference) (OtherActor :type Actor%20Object%20Reference) (OtherComp :type Primitive%20Component%20Object%20Reference) (OtherBodyIndex :type Integer) (bFromSweep :type Boolean) (SweepResult :type Hit%20Result%20Structure%20%28by%20ref%29))
  (if (not (Variables|Default|GetIsStun?))
    (bind _asbp_zombie_parent (Utilities|Casting|CastToBP_ZombieParent OtherActor))
    (Animation|Montage|PlayMontage (Variables|Default|GetSkeletalMesh) "/Game/LittleDragons/Animations/Common/LD_C_Attack_Head_Montage.LD_C_Attack_Head_Montage"
      (:OnCompleted
        (bind _newtrack_0 (Timeline|f Play)
          (:Update
            (Transformation|SetRelativeLocation (Variables|Default|GetSkeletalMesh) (Math|Vector|MakeVector 0.0 0.0 (Math|Float|Lerp 0.0 -2e+02 _newtrack_0)) false false))
          (:Finished
            (Components|Activation|Activate (Variables|/Script/Engine.Character|GetCharacterMovement _asbp_zombie_parent) false)
            (Variables|Default|SetIsStun? false)
            (Actor|DestroyActor)
            (Variables|/Game/Blueprints/Zombies/BP_ZombieParent.BP_ZombieParent_C|SetIsStun? _asbp_zombie_parent false))))
      (:OnNotifyBegin
        (Components|Activation|Deactivate (Variables|/Script/Engine.Character|GetCharacterMovement _asbp_zombie_parent))
        (Variables|Default|SetIsStun? true)
        (Variables|/Game/Blueprints/Zombies/BP_ZombieParent.BP_ZombieParent_C|SetIsStun? _asbp_zombie_parent true)))))

(event EventBeginPlay)

(event Collision|EventActorBeginOverlap
  (params (OtherActor :type Actor%20Object%20Reference)))

(event EventTick
  (params (DeltaSeconds :type Float%20%28single-precision%29)))

(fn ConstructionScript)