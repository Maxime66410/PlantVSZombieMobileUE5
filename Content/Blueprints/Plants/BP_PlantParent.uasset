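; Base plant actor that provides shared stats, damage handling and projectile firing, with empty Shoot, ImproveShootRate and RefreshAttackSpeed events as hooks.
; On BeginPlay, Attack and Hp are derived from StatsPlante, scaled by half its Level.
; Damage reduces Hp; at zero it sets Death and destroys the capsule component, leaving the actor alive.
; ShootProjectile spawns BP_ProjectileSimple at the Arrow, passing Attack as damage; Tick prints Attack and Hp for debugging.
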(event Custom|ShootProjectile
  (bind _arrow (Variables|Default|GetArrow))
  (Game|SpawnActorfromClass "/Game/Blueprints/Plants/BP_ProjectileSimple.BP_ProjectileSimple_C" (Math|Transform|MakeTransform (Transformation|GetWorldLocation _arrow) (Transformation|GetWorldRotation _arrow) "1.000000,1.000000,1.000000") "AlwaysSpawn" "MultiplyWithRoot" 0 (Variables|Default|GetAttack) false 0))

(event Custom|Shoot)

(event Custom|RefreshAttackSpeed)

(event Custom|ImproveShootRate
  (params (Rating :type Float%20%28double-precision%29)))

(event EventBeginPlay
  (CallFunction|SetStatistiqueBasique))

(event Game|Damage|EventAnyDamage
  (params (Damage :type Float%20%28single-precision%29) (DamageType :type Damage%20Type%20Object%20Reference) (InstigatedBy :type Controller%20Object%20Reference) (DamageCauser :type Actor%20Object%20Reference))
  (bind _output_get (Variables|Default|SetHp (- (Variables|Default|GetHp) Damage)))
  (if (<= _output_get 0.0)
    (Variables|Default|SetDeath? true)
    (bind _capsule (Variables|Default|GetCapsule)
      (:then
        (Components|DestroyComponent _capsule))
      (:else))))

(event EventTick
  (params (DeltaSeconds :type Float%20%28single-precision%29))
  (Development|PrintString (Utilities|String|Append (Utilities|String|ToString(Float) (Variables|Default|GetAttack)) " - " (Utilities|String|ToString(Float) (Variables|Default|GetHp))) true true "(R=0.000000,G=0.660000,B=1.000000,A=1.000000)" 0.0))

(fn ConstructionScript)

(fn SetStatistiqueBasique
  (bind _statsplante (Variables|Default|GetStatsPlante))
  (bind (_level _hp _attack) (Utilities|Struct|BreakS_StatsPlant _statsplante))
  (LocalVariables|SetCoef (* _level 0.5))
  (Variables|Default|SetAttack (* _attack (LocalVariables|GetCoef)))
  (Variables|Default|SetHp (* _hp (LocalVariables|GetCoef))))