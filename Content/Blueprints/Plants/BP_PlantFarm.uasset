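; BP_PlantFarm is a plant actor that generates gold for the player over time.
; On BeginPlay it runs the parent logic, then starts a looping ten-second timer bound to its Farm event.
; Each Farm call adds GoldGiven to the Gold variable on the first player's BP_CustomPlayerController.
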(event Custom|Farm
  (bind _returnvalue (Game|GetPlayerController 0))
  (bind _asbp_custom_player_controller (Utilities|Casting|CastToBP_CustomPlayerController _returnvalue))
  (Variables|/Game/Blueprints/BP_CustomPlayerController.BP_CustomPlayerController_C|SetGold _asbp_custom_player_controller (+ (Variables|Default|GetGoldGiven) (Variables|/Game/Blueprints/BP_CustomPlayerController.BP_CustomPlayerController_C|GetGold _asbp_custom_player_controller))))

(event EventBeginPlay
  (|CallParentFunction)
  (Utilities|Time|SetTimerbyEvent (delegate Custom|Farm) 1e+01 true))

(event Collision|EventActorBeginOverlap
  (params (OtherActor :type Actor%20Object%20Reference))
  (|CallParentFunction OtherActor) ; This node is disabled and will not be called.\nDrag off pins to build functionality.
)

(event EventTick
  (params (DeltaSeconds :type Float%20%28single-precision%29))
  (|CallParentFunction DeltaSeconds) ; This node is disabled and will not be called.\nDrag off pins to build functionality.
)

(fn ConstructionScript
  (|CallParentFunction))