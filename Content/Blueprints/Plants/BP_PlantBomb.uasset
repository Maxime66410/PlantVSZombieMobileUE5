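; BP_PlantBomb is a plant bomb that detonates on a short timer after it spawns.
; BeginPlay runs the parent logic, then sets a one-shot timer that fires Explosion.
; Explosion runs a stationary, debug-drawn box trace on Visibility around the actor and calls Death on the hit BP_ZombieParent.
; The single-hit trace affects at most one zombie, and the bomb does not destroy itself here.
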(event Custom|Explosion
  (bind _returnvalue (Transformation|GetActorLocation))
  (bind _outhit (Collision|BoxTraceByChannel _returnvalue _returnvalue "300.000000,300.000000,50.000000" "0, 0, 0" "TraceTypeQuery1" false 0 "ForDuration"))
  (bind _asbp_zombie_parent (Utilities|Casting|CastToBP_ZombieParent (.HitActor (Collision|BreakHitResult _outhit))))
  (Default|Death _asbp_zombie_parent))

(event EventBeginPlay
  (|CallParentFunction)
  (Utilities|Time|SetTimerbyEvent (delegate Custom|Explosion) 2.0))

(event Collision|EventActorBeginOverlap
  (params (OtherActor :type Actor%20Object%20Reference))
  (|CallParentFunction OtherActor) ; This node is disabled and will not be called.\nDrag off pins to build functionality.
)

(event EventTick
  (params (DeltaSeconds :type Float%20%28single-precision%29))
  (|CallParentFunction DeltaSeconds) ; This node is disabled and will not be called.\nDrag off pins to build functionality.
)

(fn ConstructionScript
  (|CallParentFunction))