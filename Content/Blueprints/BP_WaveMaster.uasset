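; BP_WaveMaster is the wave manager that runs escalating zombie waves, with a boss wave every fifth wave.
; It pools existing zombie and boss actors, teleporting them from a lobby to randomized spawn points and setting each AI blackboard's Base to a matching target point.
; HP and attack scale with wave number and reset between waves.
; A looping timer ends the wave when the live count reaches zero, then starts a delay timer.
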(event Custom|PrepareWave
  (bind (_outitem _output) (Utilities|GetRandomSpawn))
  (bind _listofzombie (Variables|Default|GetListOfZombie))
  (bind _listofzombie_2 (Variables|Default|GetListOfZombie))
  (bind _wavenbr (Variables|Default|GetWaveNbr))
  (bind _returnvalue (Utilities|Array|Length _listofzombie_2))
  (bind _returnvalue_2 (Utilities|Array|Length _listofzombie))
  (bind _returnvalue_3 (Math|Conversions|ToFloat(Integer) _wavenbr))
  (bind _returnvalue_4 (/ _returnvalue_3 2e+01))
  (bind _returnvalue_5 (+ _returnvalue_4 1.0))
  ;[0.4862 1 0.4456] Prepare Wave
  (Variables|Default|SetCurrentZombie 2)
  (CallFunction|RespawnAllZombie)
  (Utilities|FlowControl|Sequence
    (:then_0
      ;;[1 0.8088 0] Prepare Round Information
      (bind _result (Math|Integer|IncrementInt (Variables|Default|GetWaveNbr))
        (:%20%20
          (Variables|Default|SetCurrentZombie (select (>= (+ (Variables|Default|GetCurrentZombie) _result) _returnvalue) _returnvalue (+ (Variables|Default|GetCurrentZombie) _result)))
          (Development|PrintText (Utilities|Text|FormatText "WAVE PREPARATION 
Wave : {A} 
Current Zombie : {B}" (Variables|Default|GetWaveNbr) (Variables|Default|GetCurrentZombie)) true true "(R=1.000000,G=0.000000,B=0.046064,A=1.000000)"))))
    (:then_1
      ;;[1 0 0.4837] Spawn Zombie
      (for _index (range 0 (select (>= (Variables|Default|GetCurrentZombie) _returnvalue_2) (- _returnvalue_2 1) (- (Variables|Default|GetCurrentZombie) 1)))
        (Variables|Default|SetRandomIndex (Math|Random|RandomInteger (Utilities|Array|Length (Variables|Default|GetSpawnArray))))
        (Transformation|SetActorLocation (Utilities|Array|Get(acopy) (Variables|Default|GetListOfZombie) _index) _outitem false true)
        (AI|Components|Blackboard|SetValueasObject (Variables|/Script/AIModule.AIController|GetBlackboard (AI|GetAIController (Utilities|Array|Get(acopy) (Variables|Default|GetListOfZombie) _index))) (Utilities|String|StringToName "Base") _output)
        (AI|Components|Blackboard|SetValueasObject (Variables|/Script/AIModule.AIController|GetBlackboard (AI|GetAIController (Utilities|Array|Get(acopy) (Variables|Default|GetListOfZombie) _index))) (Utilities|String|StringToName "Target") 0)
        (Variables|/Game/Blueprints/Zombies/BP_ZombieParent.BP_ZombieParent_C|SetStatsZombies (Utilities|Array|Get(acopy) (Variables|Default|GetListOfZombie) _index) (Utilities|Struct|MakeS_StatsZombie (.zombietype (Variables|/Game/Blueprints/Zombies/BP_ZombieParent.BP_ZombieParent_C|GetStatsZombies (Utilities|Array|Get(acopy) (Variables|Default|GetListOfZombie) _index))) (* (.hp (Variables|/Game/Blueprints/Zombies/BP_ZombieParent.BP_ZombieParent_C|GetStatsZombies (Utilities|Array|Get(acopy) (Variables|Default|GetListOfZombie) _index))) _returnvalue_5) (* (.attack (Variables|/Game/Blueprints/Zombies/BP_ZombieParent.BP_ZombieParent_C|GetStatsZombies (Utilities|Array|Get(acopy) (Variables|Default|GetListOfZombie) _index))) _returnvalue_5) (.movespeed (Variables|/Game/Blueprints/Zombies/BP_ZombieParent.BP_ZombieParent_C|GetStatsZombies (Utilities|Array|Get(acopy) (Variables|Default|GetListOfZombie) _index))) (.score (Variables|/Game/Blueprints/Zombies/BP_ZombieParent.BP_ZombieParent_C|GetStatsZombies (Utilities|Array|Get(acopy) (Variables|Default|GetListOfZombie) _index)))))
        (Variables|/Game/Blueprints/Zombies/BP_ZombieParent.BP_ZombieParent_C|SetisDead? (Utilities|Array|Get(acopy) (Variables|Default|GetListOfZombie) _index) false))
      (if (not (Math|Conversions|ToBoolean(Integer) (Math|Integer|%(Integer) (Variables|Default|GetWaveNbr) 5)))
        (CallFunction|SpawnBossWave)
        (Development|PrintString "BOSS WAVE BEGIN" true true "(R=0.406250,G=0.000000,B=0.058921,A=1.000000)" 3.0)
        (Audio|PlaySound2D "/Game/Sounds/OrcHornBig.OrcHornBig" 1.0 1.0 0.0 0 0)
        (bind _returnvalue_6 (UserInterface|CreateWidget "/Game/Widget/WBP_BossWave.WBP_BossWave_C"))
        (UserInterface|Viewport|AddtoViewport _returnvalue_6 0)))
    (:then_2
      ;;[0.1114 0 1] Start Wave
      (if (Class|KismetSystemLibrary|TimerExistsHandle (Variables|Default|GetEvent_WaveInstanced))
        (Utilities|Time|UnpauseTimerbyHandle (Variables|Default|GetEvent_WaveInstanced))
        (else
          (bind _returnvalue_7 (Utilities|Time|SetTimerbyEvent (EventDispatchers|CreateEvent :!event Custom|Wave) 1.0 true))
          (Variables|Default|SetEvent_WaveInstanced _returnvalue_7))))))

(event Custom|Wave
  ;[1 0.4347 0] Current Wave
  (if (<= (Variables|Default|GetCurrentZombie) 0)
    (CallFunction|EndWave)
    (Utilities|Time|PauseTimerbyHandle (Variables|Default|GetEvent_WaveInstanced))))

(event Custom|EndWave
  ;[1 0 0.7769] End Wave | Reset all
  (CallFunction|RespawnAllZombie)
  (Utilities|Time|SetTimerbyEvent (EventDispatchers|CreateEvent :!event Custom|PrepareWave) 5.0)
  (Utilities|Time|PauseTimerbyHandle (Variables|Default|GetEvent_WaveInstanced))
  (Development|PrintText (Utilities|Text|FormatText "WAVE {A} ENDED" (Variables|Default|GetWaveNbr)) true true "(R=0.000000,G=1.000000,B=0.034121,A=1.000000)"))

(event EventBeginPlay
  ;[0.1094 0.03763 0.08913] Begin Play
  (CallFunction|CheckAiArray)
  (CallFunction|GetAutoTarget)
  (CallFunction|GetPosSpawn)
  (Utilities|Time|SetTimerbyEvent (EventDispatchers|CreateEvent :!event Custom|PrepareWave) 5.0))

(fn ConstructionScript)

(fn CheckAiArray
  (Utilities|FlowControl|Sequence
    (:then_0
      (if (Utilities|Array|IsEmpty (Variables|Default|GetListOfZombie))
        (Development|PrintString "WARNING : Wave Zombie is null" true true "(R=1.000000,G=0.843707,B=0.000000,A=1.000000)" 5.0)
        (bind _outactors (Actor|GetAllActorsOfClass "/Game/Blueprints/Zombies/BP_ZombieParent.BP_ZombieParent_C"))
        (Variables|Default|SetListOfZombie _outactors)))
    (:then_1
      (for _array_element (Variables|Default|GetListOfZombie)
        (Utilities|IsValid _array_element
          (:Is%20Valid
            (Variables|/Game/Blueprints/Zombies/BP_ZombieParent.BP_ZombieParent_C|SetRef_WaveMaster _array_element self)))))
    (:then_2
      (if (Utilities|Array|IsEmpty (Variables|Default|GetListOfBoss))
        (Development|PrintString "WARNING : Wave Big Zombie is null" true true "(R=1.000000,G=0.843707,B=0.000000,A=1.000000)" 5.0)
        (bind _outactors_2 (Actor|GetAllActorsOfClass "/Game/Blueprints/Zombies/BP_ZombieParent.BP_ZombieParent_C"))
        (for _array_element_2 _outactors_2
          (if (Utilities|Enum|Equal(Enum) (.zombietype (Variables|/Game/Blueprints/Zombies/BP_ZombieParent.BP_ZombieParent_C|GetStatsZombies _array_element_2)) "NewEnumerator3")
            (Utilities|Array|Add (Variables|Default|GetListOfBoss) _array_element_2)))))
    (:then_3
      (for _array_element_3 (Variables|Default|GetListOfBoss)
        (Utilities|IsValid _array_element_3
          (:Is%20Valid
            (Variables|/Game/Blueprints/Zombies/BP_ZombieParent.BP_ZombieParent_C|SetRef_WaveMaster _array_element_3 self)))))))

(fn RespawnZombie
  (params (CurrentZombie :type BP%20Zombie%20Parent%20Object%20Reference))
  (bind _returnvalue (AI|GetAIController CurrentZombie))
  (bind _returnvalue_2 (AI|GetAIController CurrentZombie))
  (bind _blackboard (Variables|/Script/AIModule.AIController|GetBlackboard _returnvalue_2))
  (bind _blackboard_2 (Variables|/Script/AIModule.AIController|GetBlackboard _returnvalue))
  (if (Utilities|Array|ContainsItem (Variables|Default|GetListOfZombie) CurrentZombie)
    (Transformation|SetActorLocation CurrentZombie (Transformation|GetWorldLocation (Variables|Default|GetSpawnLobby)) false true)
    (Math|Integer|DecrementInt (Variables|Default|GetCurrentZombie)
      (:%20%20
        (AI|Components|Blackboard|SetValueasObject _blackboard_2 (Utilities|String|StringToName "Base") 0)
        (AI|Components|Blackboard|SetValueasObject _blackboard_2 (Utilities|String|StringToName "Target") 0)))
    (elif (Utilities|Array|ContainsItem (Variables|Default|GetListOfBoss) CurrentZombie)
      (Transformation|SetActorLocation CurrentZombie (Transformation|GetWorldLocation (Variables|Default|GetSpawnLobby)) false true)
      (Math|Integer|DecrementInt (Variables|Default|GetCurrentZombie)
        (:%20%20
          (AI|Components|Blackboard|SetValueasObject _blackboard (Utilities|String|StringToName "Base") 0)
          (AI|Components|Blackboard|SetValueasObject _blackboard (Utilities|String|StringToName "Target") 0))))))

(fn RespawnAllZombie
  (for _array_element (Variables|Default|GetListOfZombie)
    (Transformation|SetActorLocation _array_element (Transformation|GetWorldLocation (Variables|Default|GetSpawnLobby)) false true)
    (AI|Components|Blackboard|SetValueasObject (Variables|/Script/AIModule.AIController|GetBlackboard (AI|GetAIController _array_element)) (Utilities|String|StringToName "Base") 0)
    (Variables|/Game/Blueprints/Zombies/BP_ZombieParent.BP_ZombieParent_C|SetStatsZombies _array_element (Utilities|Struct|MakeS_StatsZombie "NewEnumerator0" 1e+02 2e+01 1.5e+02 100))
    (AI|Components|Blackboard|SetValueasObject (Variables|/Script/AIModule.AIController|GetBlackboard (AI|GetAIController _array_element)) (Utilities|String|StringToName "Target") 0))
  (for _array_element_2 (Variables|Default|GetListOfBoss)
    (Transformation|SetActorLocation _array_element_2 (Transformation|GetWorldLocation (Variables|Default|GetSpawnLobby)) false true)
    (AI|Components|Blackboard|SetValueasObject (Variables|/Script/AIModule.AIController|GetBlackboard (AI|GetAIController _array_element_2)) (Utilities|String|StringToName "Base") 0)
    (Variables|/Game/Blueprints/Zombies/BP_ZombieParent.BP_ZombieParent_C|SetStatsZombies _array_element_2 (Utilities|Struct|MakeS_StatsZombie "NewEnumerator3" 5e+02 8e+01 8e+01 500))
    (AI|Components|Blackboard|SetValueasObject (Variables|/Script/AIModule.AIController|GetBlackboard (AI|GetAIController _array_element_2)) (Utilities|String|StringToName "Target") 0)))

(fn GetAutoTarget
  (if (Utilities|Array|IsEmpty (Variables|Default|GetListTarget))
    (Development|PrintString "WARNING : Target Point is null" true true "(R=1.000000,G=0.843707,B=0.000000,A=1.000000)" 5.0)
    (bind _outactors (Actor|GetAllActorsOfClass "/Script/Engine.TargetPoint"))
    (Variables|Default|SetListTarget _outactors)))

(fn GetPosSpawn
  (Variables|Default|SetSpawnArray (Utilities|Array|MakeArray (Transformation|GetWorldLocation (Variables|Default|GetSpawnInGame)) (Transformation|GetWorldLocation (Variables|Default|GetSpawnInGame2)) (Transformation|GetWorldLocation (Variables|Default|GetSpawnInGame3)) (Transformation|GetWorldLocation (Variables|Default|GetSpawnInGame4)) (Transformation|GetWorldLocation (Variables|Default|GetSpawnInGame5)))))

(fn SpawnBossWave
  (bind (_outitem _output) (Utilities|GetRandomSpawn))
  (bind _listofboss (Variables|Default|GetListOfBoss))
  (bind _wavenbr (Variables|Default|GetWaveNbr))
  (bind _returnvalue (Utilities|Array|Length _listofboss))
  (bind _returnvalue_2 (Math|Conversions|ToFloat(Integer) _wavenbr))
  (bind _returnvalue_3 (/ _returnvalue_2 35.0))
  (bind _returnvalue_4 (+ _returnvalue_3 1.0))
  (LocalVariables|SetRdnSpawn (Math|Random|RandomIntegerinRange 1 (Utilities|Array|Length (Variables|Default|GetListOfBoss))))
  (Variables|Default|SetCurrentZombie (+ (Variables|Default|GetCurrentZombie) (LocalVariables|GetRdnSpawn)))
  (for _index (range 0 (select (>= (LocalVariables|GetRdnSpawn) _returnvalue) (- _returnvalue 1) (- (LocalVariables|GetRdnSpawn) 1)))
    (Variables|Default|SetRandomIndex (Math|Random|RandomInteger (Utilities|Array|Length (Variables|Default|GetSpawnArray))))
    (Transformation|SetActorLocation (Utilities|Array|Get(acopy) (Variables|Default|GetListOfBoss) _index) _outitem false true)
    (AI|Components|Blackboard|SetValueasObject (Variables|/Script/AIModule.AIController|GetBlackboard (AI|GetAIController (Utilities|Array|Get(acopy) (Variables|Default|GetListOfBoss) _index))) (Utilities|String|StringToName "Base") _output)
    (AI|Components|Blackboard|SetValueasObject (Variables|/Script/AIModule.AIController|GetBlackboard (AI|GetAIController (Utilities|Array|Get(acopy) (Variables|Default|GetListOfBoss) _index))) (Utilities|String|StringToName "Target") 0)
    (Variables|/Game/Blueprints/Zombies/BP_ZombieParent.BP_ZombieParent_C|SetStatsZombies (Utilities|Array|Get(acopy) (Variables|Default|GetListOfBoss) _index) (Utilities|Struct|MakeS_StatsZombie (.zombietype (Variables|/Game/Blueprints/Zombies/BP_ZombieParent.BP_ZombieParent_C|GetStatsZombies (Utilities|Array|Get(acopy) (Variables|Default|GetListOfBoss) _index))) (* (.hp (Variables|/Game/Blueprints/Zombies/BP_ZombieParent.BP_ZombieParent_C|GetStatsZombies (Utilities|Array|Get(acopy) (Variables|Default|GetListOfBoss) _index))) _returnvalue_4) (* (.attack (Variables|/Game/Blueprints/Zombies/BP_ZombieParent.BP_ZombieParent_C|GetStatsZombies (Utilities|Array|Get(acopy) (Variables|Default|GetListOfBoss) _index))) _returnvalue_4) (.movespeed (Variables|/Game/Blueprints/Zombies/BP_ZombieParent.BP_ZombieParent_C|GetStatsZombies (Utilities|Array|Get(acopy) (Variables|Default|GetListOfBoss) _index))) (.score (Variables|/Game/Blueprints/Zombies/BP_ZombieParent.BP_ZombieParent_C|GetStatsZombies (Utilities|Array|Get(acopy) (Variables|Default|GetListOfBoss) _index)))))
    (Variables|/Game/Blueprints/Zombies/BP_ZombieParent.BP_ZombieParent_C|SetisDead? (Utilities|Array|Get(acopy) (Variables|Default|GetListOfBoss) _index) false)))