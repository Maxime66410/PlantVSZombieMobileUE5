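; AIC_Zombie is the AI controller for zombies, choosing what they target through the blackboard of BT_Zombie.
; On possess it caches the pawn as BP_ZombieParent and runs that behavior tree.
; BeginPlay sets Target to the Bp_Base actor, a step marked temporary.
; Each tick, while the zombie's IsHit is true, Target switches to the plant parent reference stored on the zombie.
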(event EventBeginPlay
  ;[0 0 0] Temporaire
  (bind _returnvalue (Actor|GetActorOfClass "/Game/Blueprints/Zombies/Bp_Base.Bp_Base_C"))
  (AI|Components|Blackboard|SetValueasObject (Variables|Default|GetBlackboard) (Utilities|String|StringToName "Target") _returnvalue))

(event EventTick
  (params (DeltaSeconds :type Float%20%28single-precision%29))
  (if (Variables|/Game/Blueprints/Zombies/BP_ZombieParent.BP_ZombieParent_C|GetIsHit? (Variables|Default|GetAs%20BP%20Zombie%20Parent))
    (AI|Components|Blackboard|SetValueasObject (Variables|Default|GetBlackboard) (Utilities|String|StringToName "Target") (Variables|/Game/Blueprints/Zombies/BP_ZombieParent.BP_ZombieParent_C|GetAs%20BP%20Plant%20Parent (Variables|Default|GetAs%20BP%20Zombie%20Parent)))))

(event EventPossess
  (params (PossessedPawn :type Pawn%20Object%20Reference))
  (bind _asbp_zombie_parent (Utilities|Casting|CastToBP_ZombieParent PossessedPawn))
  (Variables|Default|SetAs%20BP%20Zombie%20Parent _asbp_zombie_parent)
  (AI|RunBehaviorTree "/Game/Blueprints/Zombies/BT_Zombie.BT_Zombie"))

(fn ConstructionScript)