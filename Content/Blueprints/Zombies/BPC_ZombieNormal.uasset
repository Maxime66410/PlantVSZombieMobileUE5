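; BPC_ZombieNormal is a normal zombie variant that randomizes its orc appearance on construction.
; After the parent construction script, it stores a random pick of Warrior, Warlock or Hunter skeletal mesh in ChooseSkMesh.
; That index also selects the matching material sets, with armor and body each rolled independently from three options.
; The third Warlock body option uses a Warrior material, and the event graph adds no logic.
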(event EventBeginPlay)

(event Collision|EventActorBeginOverlap
  (params (OtherActor :type Actor%20Object%20Reference)))

(event EventTick
  (params (DeltaSeconds :type Float%20%28single-precision%29)))

(fn ConstructionScript
  (bind _returnvalue (Math|Random|RandomIntegerinRange 0 2))
  (bind _mesh (Variables|Character|GetMesh))
  (|CallParentFunction)
  (bind _output_get (Variables|Default|SetChooseSkMesh (Math|Random|RandomIntegerinRange 0 2)))
  (Components|SkeletalMesh|SetSkeletalMeshAsset (Variables|Character|GetMesh) (Utilities|Select :Index _output_get :Option%200 "/Game/Stylized_Orcs/Orc_Warrior/Meshes/SK_Orc_Warrior.SK_Orc_Warrior" :Option%201 "/Game/Stylized_Orcs/Orc_Warlock/Meshes/SK_Orc_Warlock.SK_Orc_Warlock" :Option%202 "/Game/Stylized_Orcs/Orc_Hunter/Meshes/SK_Orc_Hunter.SK_Orc_Hunter"))
  (Rendering|Material|SetMaterial _mesh 0 (Utilities|Select :Index (Variables|Default|GetChooseSkMesh) :Option%200 (Utilities|Select :Index _returnvalue :Option%200 "/Game/Stylized_Orcs/Orc_Warrior/Materials/Instances/MI_Warrior_Armor_1.MI_Warrior_Armor_1" :Option%201 "/Game/Stylized_Orcs/Orc_Warrior/Materials/Instances/MI_Warrior_Armor_2.MI_Warrior_Armor_2" :Option%202 "/Game/Stylized_Orcs/Orc_Warrior/Materials/Instances/MI_Warrior_Armor_3.MI_Warrior_Armor_3") :Option%201 (Utilities|Select :Index _returnvalue :Option%200 "/Game/Stylized_Orcs/Orc_Warlock/Materials/Instances/MI_Warlock_Armor_1.MI_Warlock_Armor_1" :Option%201 "/Game/Stylized_Orcs/Orc_Warlock/Materials/Instances/MI_Warlock_Armor_2.MI_Warlock_Armor_2" :Option%202 "/Game/Stylized_Orcs/Orc_Warlock/Materials/Instances/MI_Warlock_Armor_3.MI_Warlock_Armor_3") :Option%202 (Utilities|Select :Index _returnvalue :Option%200 "/Game/Stylized_Orcs/Orc_Hunter/Materials/Instances/MI_Armor1.MI_Armor1" :Option%201 "/Game/Stylized_Orcs/Orc_Hunter/Materials/Instances/MI_Armor2.MI_Armor2" :Option%202 "/Game/Stylized_Orcs/Orc_Hunter/Materials/Instances/MI_Armor3.MI_Armor3")))
  (Rendering|Material|SetMaterial _mesh 1 (Utilities|Select :Index (Variables|Default|GetChooseSkMesh) :Option%200 (Utilities|Select :Index _returnvalue :Option%200 "/Game/Stylized_Orcs/Orc_Warrior/Materials/Instances/MI_Warrior_Body_1.MI_Warrior_Body_1" :Option%201 "/Game/Stylized_Orcs/Orc_Warrior/Materials/Instances/MI_Warrior_Body_2.MI_Warrior_Body_2" :Option%202 "/Game/Stylized_Orcs/Orc_Warrior/Materials/Instances/MI_Warrior_Body_3.MI_Warrior_Body_3") :Option%201 (Utilities|Select :Index _returnvalue :Option%200 "/Game/Stylized_Orcs/Orc_Warlock/Materials/Instances/MI_Warlock_Body_1.MI_Warlock_Body_1" :Option%201 "/Game/Stylized_Orcs/Orc_Warlock/Materials/Instances/MI_Warlock_Body_2.MI_Warlock_Body_2" :Option%202 "/Game/Stylized_Orcs/Orc_Warrior/Materials/Instances/MI_Warrior_Body_3.MI_Warrior_Body_3") :Option%202 (Utilities|Select :Index _returnvalue :Option%200 "/Game/Stylized_Orcs/Orc_Hunter/Materials/Instances/MI_Body_1.MI_Body_1" :Option%201 "/Game/Stylized_Orcs/Orc_Hunter/Materials/Instances/MI_Body_2.MI_Body_2" :Option%202 "/Game/Stylized_Orcs/Orc_Hunter/Materials/Instances/MI_Body_3.MI_Body_3"))))