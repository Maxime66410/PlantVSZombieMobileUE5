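; Bp_Base is the base that zombies must not reach, ending the game in a loss on contact.
; The first BP_ZombieParent to overlap its Box shows the lose screen, swaps the gamemode's main sound for a defeat track and slows global time.
; A separate SaveScore function adds the player controller's truncated Gold to the GameInstance save and writes it, but nothing in this Blueprint calls it.
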(event OnComponentBeginOverlap(Box)
  (params (OverlappedComponent :type Primitive%20Component%20Object%20Reference) (OtherActor :type Actor%20Object%20Reference) (OtherComp :type Primitive%20Component%20Object%20Reference) (OtherBodyIndex :type Integer) (bFromSweep :type Boolean) (SweepResult :type Hit%20Result%20Structure%20%28by%20ref%29))
  (Utilities|Casting|CastToBP_ZombieParent OtherActor)
  (Utilities|FlowControl|DoOnce false
    (:Completed
      (bind _returnvalue (UserInterface|CreateWidget "/Game/Widget/Loose/WBP_LooseScreen.WBP_LooseScreen_C"))
      (UserInterface|Viewport|AddtoViewport _returnvalue 0)
      (Audio|Components|Audio|Stop (Variables|/Game/Blueprints/BP_CustomGamemode.BP_CustomGamemode_C|GetSoundMain (Variables|Default|GetAs%20BP%20Custom%20Gamemode)))
      (Audio|PlaySound2D "/Game/Sounds/LOSE_YOURSELF_｜_Medieval_Bardcore_Version_｜_8_Mile_｜_Eminem_vs_Beedle_the_Bardcore.LOSE_YOURSELF_｜_Medieval_Bardcore_Version_｜_8_Mile_｜_Eminem_vs_Beedle_the_Bardcore" 0.2 1.0 0.0 0 0)
      (Utilities|Time|SetGlobalTimeDilation 0.1))))

(event EventBeginPlay
  (bind _asbp_custom_gamemode (Utilities|Casting|CastToBP_CustomGamemode (Game|GetGameMode)))
  (Variables|Default|SetAs%20BP%20Custom%20Gamemode _asbp_custom_gamemode))

(fn ConstructionScript)

(fn SaveScore
  (bind _returnvalue (Game|GetGameInstance))
  (bind _asbp_custom_game_instance (Utilities|Casting|CastToBP_CustomGameInstance _returnvalue))
  (bind _saveref (Variables|/Game/Blueprints/BP_CustomGameInstance.BP_CustomGameInstance_C|GetSaveRef _asbp_custom_game_instance))
  (Variables|/Game/Blueprints/Save/BP_SaveCustom.BP_SaveCustom_C|SetGold _saveref (+ (Variables|/Game/Blueprints/Save/BP_SaveCustom.BP_SaveCustom_C|GetGold _saveref) (Math|Float|Truncate (Variables|/Game/Blueprints/BP_CustomPlayerController.BP_CustomPlayerController_C|GetGold (.AsBP%20Custom%20Player%20Controller (Utilities|Casting|CastToBP_CustomPlayerController (Game|GetPlayerController 0)))))))
  (Default|Save _asbp_custom_game_instance))