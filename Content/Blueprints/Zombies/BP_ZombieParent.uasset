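; BP_ZombieParent is a zombie base class driven by a stats struct for health, attack, speed and score.
; Each Tick, a debug-drawn forward line trace caches any BP_PlantParent hit and sets IsHit, which is never cleared here.
; The Apply Damage function damages that cached plant, though nothing in this file calls it.
; Incoming damage reduces health; at zero, the zombie adds score and a kill to the player controller, then destroys itself.
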(event Custom|Death
  (bind _returnvalue (Game|GetPlayerController 0))
  (bind _asbp_custom_player_controller (Utilities|Casting|CastToBP_CustomPlayerController _returnvalue))
  (Variables|/Game/Blueprints/BP_CustomPlayerController.BP_CustomPlayerController_C|SetScore _asbp_custom_player_controller (+ (.score (Variables|Default|GetStatsZombies)) (Variables|/Game/Blueprints/BP_CustomPlayerController.BP_CustomPlayerController_C|GetScore _asbp_custom_player_controller)))
  (Variables|/Game/Blueprints/BP_CustomPlayerController.BP_CustomPlayerController_C|SetKill _asbp_custom_player_controller (+ (Variables|/Game/Blueprints/BP_CustomPlayerController.BP_CustomPlayerController_C|GetKill _asbp_custom_player_controller) 1))
  (Actor|DestroyActor))

(event Game|Damage|EventAnyDamage
  (params (Damage :type Float%20%28single-precision%29) (DamageType :type Damage%20Type%20Object%20Reference) (InstigatedBy :type Controller%20Object%20Reference) (DamageCauser :type Actor%20Object%20Reference))
  (bind _output_get (Variables|Default|SetStatsZombies (Utilities|Struct|MakeS_StatsZombie (.zombietype (Variables|Default|GetStatsZombies)) (- (.hp (Variables|Default|GetStatsZombies)) Damage) (.attack (Variables|Default|GetStatsZombies)) (.movespeed (Variables|Default|GetStatsZombies)) (.score (Variables|Default|GetStatsZombies)))))
  (if (<= (.hp _output_get) 0.0)
    (CallFunction|Death)))

(event EventBeginPlay
  (Variables|/Script/Engine.CharacterMovementComponent|SetMaxWalkSpeed (Variables|Character|GetCharacterMovement) (.movespeed (Variables|Default|GetStatsZombies))))

(event EventTick
  (params (DeltaSeconds :type Float%20%28single-precision%29))
  (bind _returnvalue (Transformation|GetActorLocation))
  (bind _outhit (Collision|LineTraceByChannel _returnvalue (+ _returnvalue (* (Transformation|GetActorForwardVector) 2e+02)) "TraceTypeQuery1" false 0 "ForOneFrame"))
  (if (.bblockinghit _outhit)
    (bind _asbp_plant_parent (Utilities|Casting|CastToBP_PlantParent (.hitactor _outhit)))
    (Variables|Default|SetAs%20BP%20Plant%20Parent _asbp_plant_parent)
    (Variables|Default|SetIsHit? true)))

(fn ConstructionScript)

(fn ApplyDamage
  (Game|Damage|ApplyDamage (Variables|Default|GetAs%20BP%20Plant%20Parent) (.attack (Variables|Default|GetStatsZombies)) 0 0)
  (return))