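; BP_CustomGameInstance is a game instance that sets up the game's save data when it initializes.
; It loads the "SaveGame" slot into SaveRef as a BP_SaveCustom, or creates a new save object in memory when none exists.
; It then prints the inventory length and gold from that save.
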(event EventInit
  (Utilities|FlowControl|Sequence
    (:then_0
      (bind _returnvalue (SaveGame|DoesSaveGameExist "SaveGame"))
      (if _returnvalue
        (bind _returnvalue_2 (SaveGame|LoadGamefromSlot "SaveGame"))
        (bind _asbp_save_custom (Utilities|Casting|CastToBP_SaveCustom _returnvalue_2))
        (Variables|Default|SetSaveRef _asbp_save_custom)
        (else
          (bind _returnvalue_3 (SaveGame|CreateSaveGameObject "/Game/Blueprints/Save/BP_SaveCustom.BP_SaveCustom_C"))
          (Variables|Default|SetSaveRef _returnvalue_3))))
    (:then_1
      (Development|PrintText (Utilities|Text|FormatText "Inv Slot : {A} 
Gold : {B}" (Utilities|String|ToString(Integer) (Utilities|Array|Length (Variables|/Game/Blueprints/Save/BP_SaveCustom.BP_SaveCustom_C|GetInventaire (Variables|Default|GetSaveRef)))) (Variables|/Game/Blueprints/Save/BP_SaveCustom.BP_SaveCustom_C|GetGold (Variables|Default|GetSaveRef)))))))