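; BP_Egg is a plant egg that drops, hatches and spawns the plant matching its TypePlant.
; A timeline, with no trigger wired in this graph, lowers the Egg mesh, then starts the hatch montage.
; The selected plant class spawns just above the egg as the montage starts, and its End notify destroys the egg.
; The construction script and SetPlantType pick egg materials by type, using differing mappings.
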(fn ConstructionScript
  (Rendering|Material|SetMaterial (Variables|Default|GetEgg) 0 (Utilities|Select :Index (Variables|Default|GetTypePlant) :NewEnumerator3 "/Game/LittleDragons/Materials/Eggs/Mat_Egg_BlueMarine.Mat_Egg_BlueMarine" :NewEnumerator0 "/Game/LittleDragons/Materials/Eggs/Mat_Egg_Magnenta.Mat_Egg_Magnenta" :NewEnumerator1 "/Game/LittleDragons/Materials/Eggs/Mat_Egg_Red.Mat_Egg_Red" :NewEnumerator2 "/Game/LittleDragons/Materials/Eggs/Mat_Egg_Orange.Mat_Egg_Orange" :NewEnumerator4 0 :NewEnumerator5 0 :NewEnumerator6 0 :NewEnumerator7 0 :NewEnumerator8 0 :NewEnumerator9 0 :NewEnumerator10 0)))

(fn SetPlantType
  (params (TypePlant :type E_PlantType%20Enum :default "NewEnumerator3"))
  (bind _output_get (Variables|Default|SetTypePlant TypePlant))
  (Rendering|Material|SetMaterial (Variables|Default|GetEgg) 0 (Utilities|Select :Index _output_get :NewEnumerator3 "/Game/LittleDragons/Materials/Eggs/Mat_Egg_BlueMarine.Mat_Egg_BlueMarine" :NewEnumerator0 "/Game/LittleDragons/Materials/Eggs/Mat_Egg_SimplePlant.Mat_Egg_SimplePlant" :NewEnumerator1 "/Game/LittleDragons/Materials/Eggs/Mat_Egg_BlueMarine.Mat_Egg_BlueMarine" :NewEnumerator2 "/Game/LittleDragons/Materials/Eggs/Mat_Egg_FarmPlant.Mat_Egg_FarmPlant" :NewEnumerator4 "/Game/LittleDragons/Materials/Eggs/Mat_Egg_DoubleShoot.Mat_Egg_DoubleShoot" :NewEnumerator5 "/Game/LittleDragons/Materials/Eggs/Mat_Egg_Grey.Mat_Egg_Grey" :NewEnumerator6 "/Game/LittleDragons/Materials/Eggs/Mat_Egg_Cotte.Mat_Egg_Cotte" :NewEnumerator7 "/Game/LittleDragons/Materials/Eggs/Mat_Egg_Pink.Mat_Egg_Pink" :NewEnumerator8 "/Game/LittleDragons/Materials/Eggs/Mat_Egg_Slow.Mat_Egg_Slow" :NewEnumerator9 "/Game/LittleDragons/Materials/Eggs/Mat_Egg_Green.Mat_Egg_Green" :NewEnumerator10 "/Game/LittleDragons/Materials/Eggs/Mat_Egg_Wind.Mat_Egg_Wind")))