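; Player controller for placing dragon eggs on a tile grid by touch, paid with Soleil currency.
; While dragging, an Enhanced Input touch action projects the cursor hit onto GridRef, selects that tile and colors it using a vertical trace.
; On release, it checks cost, dragon type and tile occupancy, then spawns a typed BP_Egg and deducts the price.
; Failed placements clear the selection and play force feedback.
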(event Custom|CancelDragons
  (Default|SetColorGrid (Variables|Default|GetGridRef) true)
  (Default|SetSelectedTile (Variables|Default|GetGridRef) -1 -1)
  (Game|Feedback|PlayDynamicForceFeedback 0.05 0.2 true true true true))

(event Input|EnhancedActionEvents|EnhancedInputActionIA_Touch
  (params (ActionValue :type Boolean) (ElapsedSeconds :type Float%20%28double-precision%29) (TriggeredSeconds :type Float%20%28double-precision%29) (InputAction :type Input%20Action%20Object%20Reference :default "/Game/Input/Action/IA_Touch.IA_Touch"))
  (bind _hitresult (Game|Player|GetHitResultUnderCursorbyChannel "TraceTypeQuery1" true))
  (bind _gridref (Variables|Default|GetGridRef))
  (bind _gridref_2 (Variables|Default|GetGridRef))
  (bind _location (Collision|BreakHitResult _hitresult))
  (:Triggered
    (if (and (Variables|Default|GetDragonCanBePlaced?) (Utilities|Operators|NotEqual(!=) :A _location))
      (bind _output_get (Variables|Default|SetUnderFingerLocation _location))
      (bind (_valid_ _row _column) (Default|LocationtoTile _gridref _output_get))
      (if _valid_
        (Default|SetSelectedTile _gridref _row _column)
        (bind _gridlocation (Default|TiletoGridLocation _gridref _row _column true))
        (bind _returnvalue (Collision|LineTraceByChannel (+ (Math|Conversions|ToVector(Vector2D) _gridlocation 3.1e+02) "0.000000,0.000000,1000.000000") (- (Math|Conversions|ToVector(Vector2D) _gridlocation 3.1e+02) "0.000000,0.000000,200.000000") "TraceTypeQuery4" false 0 "None"))
        (Default|SetColorGrid (Variables|Default|GetGridRef) _returnvalue))))
  (:Started
    (Development|PrintString "Hello"))
  (:Completed
    (if (and (Variables|Default|GetDragonCanBePlaced?) (>= (Variables|Collectable|GetSoleil) (.Prix (Utilities|Struct|BreakS_StatsPlant (Variables|Default|GetDragonToSpawn)))))
      (if (Utilities|Enum|NotEqual(Enum) (Utilities|Struct|BreakS_StatsPlant (Variables|Default|GetDragonToSpawn)) "NewEnumerator3")
        (bind (_valid__2 _row_2 _column_2) (Default|LocationtoTile _gridref_2 (Variables|Default|GetUnderFingerLocation)))
        (if _valid__2
          (bind _gridlocation_2 (Default|TiletoGridLocation _gridref_2 _row_2 _column_2 true))
          (bind _returnvalue_2 (Collision|LineTraceByChannel (+ (Math|Conversions|ToVector(Vector2D) _gridlocation_2 3.1e+02) "0.000000,0.000000,1000.000000") (- (Math|Conversions|ToVector(Vector2D) _gridlocation_2 3.1e+02) "0.000000,0.000000,200.000000") "TraceTypeQuery4" false (Utilities|Array|MakeArray (Variables|Default|GetGridRef)) "None"))
          (if (not _returnvalue_2)
            (bind _returnvalue_3 (Game|SpawnActorfromClass "/Game/Blueprints/BP_Egg.BP_Egg_C" (Math|Transform|MakeTransform (Math|Conversions|ToVector(Vector2D) _gridlocation_2 3.1e+02) "0, 0, 0" "1.000000,1.000000,1.000000") "AlwaysSpawn" "MultiplyWithRoot" 0 "NewEnumerator3" 0))
            (Default|SetPlantType _returnvalue_3 (Utilities|Struct|BreakS_StatsPlant (Variables|Default|GetDragonToSpawn)))
            (Variables|Collectable|SetSoleil (Math|Float|Truncate (- (Variables|Collectable|GetSoleil) (Utilities|Struct|BreakS_StatsPlant (Variables|Default|GetDragonToSpawn)))))
            (Default|SetSelectedTile (Variables|Default|GetGridRef) -1 -1)
            (Variables|Default|SetDragonCanBePlaced? true)
            (else
              (CallFunction|CancelDragons)))
          (else
            (CallFunction|CancelDragons)))
        (else
          (CallFunction|CancelDragons)))
      (else
        (CallFunction|CancelDragons)))))

(event EventBeginPlay
  (bind _returnvalue (PlayerController|LocalPlayerSubsystems|GetEnhancedInputLocalPlayerSubsystem))
  (Variables|/Script/Engine.PlayerController|SetbShowMouseCursor (Game|GetPlayerController 0) true)
  (Utilities|IsValid _returnvalue
    (:Is%20Valid
      (Input|AddMappingContext _returnvalue "/Game/Input/IMC_MobileDefault.IMC_MobileDefault" 0 "(bIgnoreAllPressedKeysUntilRelease=True,bForceImmediately=False,bNotifyUserSettings=False)"))))

(fn ConstructionScript)