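; Village placement grid actor that builds a tile grid and highlights the tiles under a selection box as valid or invalid.
; Construction fills an instanced mesh from grid dimensions and tile size; BeginPlay registers the grid with the village player controller.
; SelectTiles restores the previous selection, then moves overlapping instances to a selection mesh, colored invalid on a hit or too few tiles.
; RemoveTiles returns selected instances to the normal mesh.
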(event EventBeginPlay
  (Variables|/Game/Blueprints/Village/Bp_VillageCustomController.Bp_VillageCustomController_C|SetGrilleRef (.AsBp%20Village%20Custom%20Controller (Utilities|Casting|CastToBp_VillageCustomController (Game|GetPlayerController 0))) self))

(fn ConstructionScript
  (Utilities|FlowControl|Sequence
    (:then_0
      (for _index (range 0 (- (Variables|Default|GetGridX) 1))
        (for _index_2 (range 0 (- (Variables|Default|GetGridY) 1))
          (Components|InstancedStaticMesh|AddInstance (Variables|Default|GetNormalMesh) (Math|Transform|MakeTransform (Math|Vector|MakeVector (Math|Conversions|ToFloat(Integer) (* _index (Variables|Default|GetTileSize))) (Math|Conversions|ToFloat(Integer) (* _index_2 (Variables|Default|GetTileSize))) 0.0)) false))))))

(fn SelectTiles
  (params (Location :type Vector) (InVec :type Vector) (HitSelect? :type Boolean) (TotalCase :type Integer))
  (bind _selectedmesh_0 (Variables|Default|GetSelectedMesh_0))
  (bind _normalmesh (Variables|Default|GetNormalMesh))
  (bind _returnvalue (Class|InstancedStaticMeshComponent|GetInstancesOverlappingBox _normalmesh (Math|Box|MakeBox Location InVec) true))
  (CallFunction|SelectTileTransform (Variables|Default|GetTileSelect) _selectedmesh_0 (Variables|Default|GetNormalMesh))
  (Components|InstancedStaticMesh|ClearInstances (Variables|Default|GetSelectedMesh_0))
  (bind _instancesadd (CallFunction|SelectTileTransform _returnvalue (Variables|Default|GetNormalMesh) (Variables|Default|GetSelectedMesh_0)))
  (bind _output_get (Variables|Default|SetTileSelect _instancesadd))
  (Rendering|Material|SetMaterial _selectedmesh_0 0 (select (or (< (Utilities|Array|Length _output_get) TotalCase) HitSelect?) "/Game/Materials/Village/MI_VillageTileSelectInvalid.MI_VillageTileSelectInvalid" "/Game/Materials/Village/MI_VillageTileSelectValid.MI_VillageTileSelectValid"))
  (Class|InstancedStaticMeshComponent|RemoveInstances _normalmesh _returnvalue))

(fn SelectTileTransform
  (params (Array :type Array%20of%20Integers) (TargetGetTransform :type Instanced%20Static%20Mesh%20Component%20Object%20Reference) (TargetAddInstances :type Instanced%20Static%20Mesh%20Component%20Object%20Reference))
  (for _array_element Array
    (Utilities|Array|Add (LocalVariables|GetNewLocalVar_0) (.OutInstanceTransform (Components|InstancedStaticMesh|GetInstanceTransform TargetGetTransform _array_element true))))
  (bind _returnvalue (Components|InstancedStaticMesh|AddInstances TargetAddInstances (LocalVariables|GetNewLocalVar_0) true true))
  (return _returnvalue))

(fn RemoveTiles
  (bind _selectedmesh_0 (Variables|Default|GetSelectedMesh_0))
  (bind _tileselect (Variables|Default|GetTileSelect))
  (CallFunction|SelectTileTransform _tileselect _selectedmesh_0 (Variables|Default|GetNormalMesh))
  (Components|InstancedStaticMesh|ClearInstances _selectedmesh_0)
  (Utilities|Array|Clear _tileselect))