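; Player controller for the village screen that sets up mobile input and the village HUD, and restores saved buildings on BeginPlay.
; A touch box-traces the hit point and, if clear, spawns a Bp_Batiment there, adds it to the game instance's village save and saves.
; FindInArray replaces an existing building entry in that saved array and saves again.
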(event Input|EnhancedActionEvents|EnhancedInputActionIA_Touch
  (params (ActionValue :type Boolean) (ElapsedSeconds :type Float%20%28double-precision%29) (TriggeredSeconds :type Float%20%28double-precision%29) (InputAction :type Input%20Action%20Object%20Reference :default "/Game/Input/Action/IA_Touch.IA_Touch"))
  (bind _instanceref (Variables|Default|GetInstanceRef))
  (:Started
    (Variables|Default|SetCusorHitLocation (.Location (Collision|BreakHitResult (.HitResult (Game|Player|GetHitResultUnderCursorbyChannel "TraceTypeQuery1" true)))))
    (bind _returnvalue (Collision|BoxTraceByChannel (Variables|Default|GetCusorHitLocation) (Variables|Default|GetCusorHitLocation) (/ (Variables|Default|GetSizeMesh) 2) "0, 0, 0" "TraceTypeQuery5" false 0 "ForDuration"))
    (if (not _returnvalue)
      (bind _output_get (Variables|Default|SetS%20Batiment (Utilities|Struct|MakeS_Batiment (Variables|Default|GetCusorHitLocation) (Math|DateTime|Now) "NewEnumerator2")))
      (Game|SpawnActorfromClass "/Game/Blueprints/Village/Batiments/Bp_Batiment.Bp_Batiment_C" (Math|Transform|MakeTransform (Variables|Default|GetCusorHitLocation) "0.000000,90.000000,0.000000") "Undefined" "MultiplyWithRoot" 0 _output_get 0)
      (Utilities|Array|AddUnique (Variables|/Game/Blueprints/Save/BP_VillageSave.BP_VillageSave_C|GetBatiment (Variables|/Game/Blueprints/BP_CustomGameInstance.BP_CustomGameInstance_C|GetVillageSaveRef _instanceref)) _output_get)
      (Default|VillageSave _instanceref))))

(event EventBeginPlay
  (bind _returnvalue (PlayerController|LocalPlayerSubsystems|GetEnhancedInputLocalPlayerSubsystem))
  (Variables|/Script/Engine.PlayerController|SetbShowMouseCursor (Game|GetPlayerController 0) true)
  (Utilities|IsValid _returnvalue
    (:Is%20Valid
      (Input|AddMappingContext _returnvalue "/Game/Input/IMC_MobileDefault.IMC_MobileDefault" 0 "(bIgnoreAllPressedKeysUntilRelease=True,bForceImmediately=False,bNotifyUserSettings=False)")
      (Variables|Default|SetInstanceRef (.AsBP%20Custom%20Game%20Instance (Utilities|Casting|CastToBP_CustomGameInstance (Game|GetGameInstance))))
      (bind _returnvalue_2 (UserInterface|CreateWidget "/Game/Blueprints/Village/UI/WBP_HUDVillage.WBP_HUDVillage_C"))
      (UserInterface|Viewport|AddtoViewport _returnvalue_2 0)
      (for _array_element (Variables|/Game/Blueprints/Save/BP_VillageSave.BP_VillageSave_C|GetBatiment (Variables|/Game/Blueprints/BP_CustomGameInstance.BP_CustomGameInstance_C|GetVillageSaveRef (Variables|Default|GetInstanceRef)))
        (Game|SpawnActorfromClass "/Game/Blueprints/Village/Batiments/Bp_Batiment.Bp_Batiment_C" (Math|Transform|MakeTransform (.Location (Utilities|Struct|BreakS_Batiment _array_element)) "0.000000,90.000000,0.000000") "Undefined" "MultiplyWithRoot" 0 _array_element 0)))))

(fn ConstructionScript)

(fn FindinArray
  (params (Before%20Batiment :type S%20Batiment%20Structure) (AfterBattiment :type S%20Batiment%20Structure%20%28by%20ref%29))
  (bind _instanceref (Variables|Default|GetInstanceRef))
  (bind _villagesaveref (Variables|/Game/Blueprints/BP_CustomGameInstance.BP_CustomGameInstance_C|GetVillageSaveRef _instanceref))
  (bind _batiment (Variables|/Game/Blueprints/Save/BP_VillageSave.BP_VillageSave_C|GetBatiment _villagesaveref))
  (Utilities|Array|SetArrayElem _batiment (Utilities|Array|FindItem _batiment Before%20Batiment) AfterBattiment)
  (Default|VillageSave (Variables|Default|GetInstanceRef))
  (return AfterBattiment))