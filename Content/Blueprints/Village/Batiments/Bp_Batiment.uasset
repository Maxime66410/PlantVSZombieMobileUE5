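; Village building actor whose mesh and tap behavior follow its type, with a construction widget and timer that validates it on completion.
; Tapping Gold buildings credits gold from elapsed time; Dragon buildings open the HUD to assign a dragon, then yield dragon orbs after a delay.
; State changes update the village controller's building array, using timestamps to resume dragon timers on BeginPlay.
; Finished dragon timers apply a ready-to-collect overlay and schedule a local notification.
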(event OnClicked(StaticMesh)
  (params (TouchedComponent :type Primitive%20Component%20Object%20Reference) (ButtonPressed :type Key%20Structure :default "None"))
  (if (Variables|Default|GetIsValidBatiment)
    (switch Utilities|FlowControl|Switch|SwitchonE_TypeBatiment (Utilities|Struct|BreakS_Batiment (Variables|Default|GetBatiment))
      (:NewEnumerator1
        (CallFunction|BatimentGold))
      (:NewEnumerator2
        (CallFunction|BatimentDragon)))))

(event Custom|Construction
  (bind _returnvalue (Utilities|Time|SetTimerbyEvent (delegate Custom|EndConstruction) 1e+01))
  (Variables|Default|SetTimerConstruction _returnvalue)
  (bind _returnvalue_2 (AddComponent|AddWidgetComponent false))
  (bind _aswbp_village_construction (Utilities|Casting|CastToWBP_VillageConstruction (UserInterface|GetWidget _returnvalue_2)))
  (Variables|/Game/Blueprints/Village/UI/WBP_VillageConstruction.WBP_VillageConstruction_C|SetBatiment _aswbp_village_construction self))

(event Custom|AddDragon
  (params (Dragon :type S%20Stats%20Plant%20Structure))
  (bind _batiment (Default|FindinArray (.AsBp%20Village%20Custom%20Controller (Utilities|Casting|CastToBp_VillageCustomController (Game|GetPlayerController 0))) (Variables|Default|GetBatiment) (Utilities|Struct|MakeS_Batiment "None" (.Location (Utilities|Struct|BreakS_Batiment (Variables|Default|GetBatiment))) (Math|DateTime|Now) Dragon (.TypeBatiment (Utilities|Struct|BreakS_Batiment (Variables|Default|GetBatiment))) true 0 0)))
  (Variables|Default|SetBatiment _batiment)
  (Utilities|Time|SetTimerbyEvent (delegate Custom|CanCollect) (Math|Timespan|GetTotalSeconds (Math|Timespan|MakeTimespan 0 0 0 5 0))))

(event Custom|CanCollect
  (bind _returnvalue (Rendering|Material|CreateDynamicMaterialInstance "/Game/Materials/Village/MI_VillageReadyToCollect.MI_VillageReadyToCollect" "None" "None" :!class /Script/Engine.KismetMaterialLibrary))
  (Rendering|Material|SetOverlayMaterial (Variables|Default|GetStaticMesh) _returnvalue :!class /Script/Engine.MeshComponent)
  (Class|KismetSystemLibrary|RegisterforRemoteNotifications)
  (bind (_notificationlaunchedapp _activationevent) (Class|BlueprintPlatformLibrary|GetLaunchNotification))
  (if _notificationlaunchedapp
    (Development|PrintString _activationevent)
    (else
      (Class|BlueprintPlatformLibrary|ScheduleLocalNotificationfromNow 1 (Utilities|Text|MakeLiteralText "Votre dragon a terminé !") (Utilities|Text|MakeLiteralText "Venez récupérer vos récompenses") (Utilities|Text|MakeLiteralText "Truc de fou") "42"))))

(event Custom|EndConstruction
  (Variables|Default|SetIsValidBatiment true))

(event EventBeginPlay
  (bind _returnvalue (Math|Timespan|GetTotalSeconds (Math|Timespan|MakeTimespan 0 0 0 5 0)))
  (bind _returnvalue_2 (CallFunction|GetDiffTime))
  (bind _batiment (Variables|Default|GetBatiment))
  (bind (_typebatiment _getadragon_) (Utilities|Struct|BreakS_Batiment _batiment))
  (bind _returnvalue_3 (- _returnvalue _returnvalue_2))
  (CallFunction|Construction)
  (if (Variables|Default|GetIsValidBatiment)
    (if (and (Utilities|Enum|Equal(Enum) _typebatiment "NewEnumerator2") _getadragon_)
      (Development|PrintString (Utilities|String|ToString(Float) _returnvalue_3))
      (if (<= _returnvalue_3 0.0)
        (bind _returnvalue_4 (Rendering|Material|CreateDynamicMaterialInstance "/Game/Materials/Village/MI_VillageReadyToCollect.MI_VillageReadyToCollect" "None" "None" :!class /Script/Engine.KismetMaterialLibrary))
        (Rendering|Material|SetOverlayMaterial (Variables|Default|GetStaticMesh) _returnvalue_4 :!class /Script/Engine.MeshComponent)
        (else
          (Utilities|Time|SetTimerbyEvent (delegate Custom|CanCollect) _returnvalue_3))))))

(event EventActorOnInputTouchEnter
  (params (FingerIndex :type ETouchIndex%20Enum :default "Touch1"))
  (if (Variables|Default|GetIsValidBatiment)
    (switch Utilities|FlowControl|Switch|SwitchonE_TypeBatiment (Utilities|Struct|BreakS_Batiment (Variables|Default|GetBatiment))
      (:NewEnumerator1
        (CallFunction|BatimentGold))
      (:NewEnumerator2
        (CallFunction|BatimentDragon)))))

(event EventActorOnInputTouchEnd
  (params (FingerIndex :type ETouchIndex%20Enum :default "Touch1"))
  (if (Variables|Default|GetIsValidBatiment)
    (switch Utilities|FlowControl|Switch|SwitchonE_TypeBatiment (Utilities|Struct|BreakS_Batiment (Variables|Default|GetBatiment))
      (:NewEnumerator1
        (CallFunction|BatimentGold))
      (:NewEnumerator2
        (CallFunction|BatimentDragon)))))

(fn ConstructionScript
  (Components|StaticMesh|SetStaticMesh (Variables|Default|GetStaticMesh) (Utilities|Select :Index (.TypeBatiment (Utilities|Struct|BreakS_Batiment (Variables|Default|GetBatiment))) :NewEnumerator0 "/Engine/BasicShapes/Cone.Cone" :NewEnumerator1 "/Game/Assets/PolygonKnights/Meshes/Buildings/SM_Bld_House_RoomRound_02.SM_Bld_House_RoomRound_02" :NewEnumerator2 "/Game/Assets/PolygonKnights/Meshes/Snow/SM_Bld_House_Room_07_Snow.SM_Bld_House_Room_07_Snow" :NewEnumerator3 0)))

(fn AddOrbeDuDragon
  (bind _returnvalue (Game|GetGameInstance))
  (bind _asbp_custom_game_instance (Utilities|Casting|CastToBP_CustomGameInstance _returnvalue))
  (bind _saveref (Variables|/Game/Blueprints/BP_CustomGameInstance.BP_CustomGameInstance_C|GetSaveRef _asbp_custom_game_instance))
  (Variables|/Game/Blueprints/Save/BP_SaveCustom.BP_SaveCustom_C|SetOrbeDuDragon _saveref (+ (Math|Float|Round (CallFunction|GetDiffTime)) (Variables|/Game/Blueprints/Save/BP_SaveCustom.BP_SaveCustom_C|GetOrbeDuDragon _saveref)))
  (Default|SavePVZ _asbp_custom_game_instance))

(fn GetDiffTime
  (return (Math|Timespan|GetTotalSeconds (- (Math|DateTime|Now) (Utilities|Struct|BreakS_Batiment (Variables|Default|GetBatiment))))))

(fn CollectDragon
  (bind _returnvalue (Game|GetPlayerController 0))
  (bind _asbp_village_custom_controller (Utilities|Casting|CastToBp_VillageCustomController _returnvalue))
  (bind _batiment (Default|FindinArray _asbp_village_custom_controller (Variables|Default|GetBatiment) (Utilities|Struct|MakeS_Batiment "None" (.Location (Utilities|Struct|BreakS_Batiment (Variables|Default|GetBatiment))) (.Time (Utilities|Struct|BreakS_Batiment (Variables|Default|GetBatiment))) (Variables|/Game/Blueprints/Village/Bp_VillageCustomController.Bp_VillageCustomController_C|GetPlantSelect _asbp_village_custom_controller) (.TypeBatiment (Utilities|Struct|BreakS_Batiment (Variables|Default|GetBatiment))) false 0 0)))
  (Variables|Default|SetBatiment _batiment))

(fn BatimentDragon
  (bind _returnvalue (Game|GetPlayerController 0))
  (bind _asbp_village_custom_controller (Utilities|Casting|CastToBp_VillageCustomController _returnvalue))
  (if (not (.GetADragon? (Utilities|Struct|BreakS_Batiment (Variables|Default|GetBatiment))))
    (Default|ShowHUD _asbp_village_custom_controller self)
    (elif (>= (CallFunction|GetDiffTime) (Math|Timespan|GetTotalSeconds (Math|Timespan|MakeTimespan 0 0 0 5 0)))
      (CallFunction|AddOrbeDuDragon)
      (bind _batiment (Default|FindinArray _asbp_village_custom_controller (Variables|Default|GetBatiment) (Utilities|Struct|MakeS_Batiment (.Nom (Utilities|Struct|BreakS_Batiment (Variables|Default|GetBatiment))) (.Location (Utilities|Struct|BreakS_Batiment (Variables|Default|GetBatiment))) (.Time (Utilities|Struct|BreakS_Batiment (Variables|Default|GetBatiment))) "(Name_17_31E5F5C0489563E39149A1844FE82069=\"\",Level_26_C5EC49304D66DE75F5E6F282784B95A4=1,NombrePersonnage_36_E620521E42F2DE32A22F24B83699027B=1,Hp_7_ED1B204743CBE88A84A29F82AE91155D=1.000000,Attack_8_AA279E9241490DD875A7458F808C8501=1.000000,Prix_9_C531579B4328F404D3D57A8D694C884C=0.000000,ShootRate_15_DC7211454D4B472E2981C589DAA14134=1.000000,Slow_31_00A75B3C4CD8A83F3B5BB1B4CACEDE80=False,Image_20_909A49304C5D975846D0EFB0515A982D=None,Rareté_23_8F7902014ADAA07ED7778ABE9C5A0A8A=NewEnumerator0,ShooterType_39_53A79B434ED6A017C1829096D86644FA=NewEnumerator0,TypeDePlante_42_3BE74C8449244EA4AC60369B9675DECC=NewEnumerator3,imageInGame_45_29677908413A31E102216C994373BCED=None)" (.TypeBatiment (Utilities|Struct|BreakS_Batiment (Variables|Default|GetBatiment))) false (.Prix (Utilities|Struct|BreakS_Batiment (Variables|Default|GetBatiment))) (.Image (Utilities|Struct|BreakS_Batiment (Variables|Default|GetBatiment))) (.SizeX (Utilities|Struct|BreakS_Batiment (Variables|Default|GetBatiment))) (.SizeY (Utilities|Struct|BreakS_Batiment (Variables|Default|GetBatiment))))))
      (Variables|Default|SetBatiment _batiment)
      (Rendering|Material|SetOverlayMaterial (Variables|Default|GetStaticMesh) 0 :!class /Script/Engine.MeshComponent)
      (else
        (Development|PrintString "Pas assez de temps écoulé")))))

(fn BatimentGold
  (bind _returnvalue (Game|GetGameInstance))
  (bind _returnvalue_2 (Math|DateTime|Now))
  (bind _batiment (Variables|Default|GetBatiment))
  (bind (_nom _location _time _dragon _typebatiment _getadragon_ _prix _image _sizex _sizey) (Utilities|Struct|BreakS_Batiment _batiment))
  (bind _asbp_custom_game_instance (Utilities|Casting|CastToBP_CustomGameInstance _returnvalue))
  (bind _villagesaveref (Variables|/Game/Blueprints/BP_CustomGameInstance.BP_CustomGameInstance_C|GetVillageSaveRef _asbp_custom_game_instance))
  (Variables|/Game/Blueprints/Save/BP_VillageSave.BP_VillageSave_C|SetGold _villagesaveref (+ (Variables|/Game/Blueprints/Save/BP_VillageSave.BP_VillageSave_C|GetGold _villagesaveref) (Math|Float|Round (CallFunction|GetDiffTime))))
  (Default|SetEleminArray (.AsBp%20Village%20Custom%20Controller (Utilities|Casting|CastToBp_VillageCustomController (Game|GetPlayerController 0))) _batiment (Utilities|Struct|MakeS_Batiment _nom _location _returnvalue_2 _dragon _typebatiment _getadragon_ _prix _image _sizex _sizey))
  (Utilities|Struct|SetmembersinS_Batiment _batiment _returnvalue_2))