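; Clickable sun actor (Soleil) that, on click or touch enter, slides once toward the gold counter in the UI.
; It creates WBP_UI on BeginPlay and deprojects the NbrGold widget's screen centre to a world direction.
; A timeline lerps the actor from its current location along that direction, keeping Z fixed.
; Debug prints remain, including DT_Plantes row names, cached at construction and printed every tick.
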(event OnInputTouchEnter(Sphere)
  (params (FingerIndex :type ETouchIndex%20Enum :default "Touch1") (TouchedComponent :type Primitive%20Component%20Object%20Reference))
  (Development|PrintString (Utilities|GetDisplayName TouchedComponent)))

(event EventBeginPlay
  (Variables|/Script/Engine.PlayerController|SetbShowMouseCursor (Game|GetPlayerController 0) true)
  (bind _returnvalue (UserInterface|CreateWidget "/Game/Blueprints/UI/WBP_UI.WBP_UI_C"))
  (Variables|Default|SetNewVar _returnvalue)
  (UserInterface|Viewport|AddtoViewport _returnvalue 0))

(event Collision|EventActorBeginOverlap
  (params (OtherActor :type Actor%20Object%20Reference)))

(event EventActorOnInputTouchEnter
  (params (FingerIndex :type ETouchIndex%20Enum :default "Touch1"))
  (bind _returnvalue (Transformation|GetActorLocation))
  (bind _returnvalue_2 (Game|GetPlayerController 0))
  (bind _newvar (Variables|Default|GetNewVar))
  (bind _nbrgold (Variables|/Game/Blueprints/UI/WBP_UI.WBP_UI_C|GetNbrGold _newvar))
  (bind _returnvalue_3 (Class|Widget|GetTickSpaceGeometry _nbrgold))
  (bind _pixelposition (Class|SlateBlueprintLibrary|LocaltoViewport _returnvalue_3))
  (bind _returnvalue_4 (Class|SlateBlueprintLibrary|GetAbsoluteSize _returnvalue_3))
  (bind _returnvalue_5 (/ _returnvalue_4 2.0))
  (bind _returnvalue_6 (+ _pixelposition _returnvalue_5))
  (bind _worlddirection (Class|GameplayStatics|DeprojectScreentoWorld _returnvalue_2 _returnvalue_6))
  (bind _returnvalue_7 (* _worlddirection 2e+01))
  (bind _returnvalue_8 (+ _returnvalue _returnvalue_7))
  (Utilities|FlowControl|DoOnce false
    (:Completed
      (bind _alpha (Timeline|TransitionLocation Play)
        (:Update
          (Transformation|SetActorLocation (Math|Vector|Lerp(Vector) _returnvalue (Math|Vector|MakeVector (.x _returnvalue_8) (.y _returnvalue_8) (.Z (Math|Vector|BreakVector _returnvalue))) _alpha) false false))
        (:Finished
          (Development|PrintString "Hello"))))))

(event EventTick
  (params (DeltaSeconds :type Float%20%28single-precision%29))
  (for _array_element (Variables|Default|GetOut%20Row%20Names)
    (Development|PrintString (Utilities|String|ToString(Name) _array_element))))

(event MouseInput|EventActorOnClicked
  (params (ButtonPressed :type Key%20Structure :default "None"))
  (bind _returnvalue (Transformation|GetActorLocation))
  (bind _returnvalue_2 (Game|GetPlayerController 0))
  (bind _newvar (Variables|Default|GetNewVar))
  (bind _nbrgold (Variables|/Game/Blueprints/UI/WBP_UI.WBP_UI_C|GetNbrGold _newvar))
  (bind _returnvalue_3 (Class|Widget|GetTickSpaceGeometry _nbrgold))
  (bind _pixelposition (Class|SlateBlueprintLibrary|LocaltoViewport _returnvalue_3))
  (bind _returnvalue_4 (Class|SlateBlueprintLibrary|GetAbsoluteSize _returnvalue_3))
  (bind _returnvalue_5 (/ _returnvalue_4 2.0))
  (bind _returnvalue_6 (+ _pixelposition _returnvalue_5))
  (bind _worlddirection (Class|GameplayStatics|DeprojectScreentoWorld _returnvalue_2 _returnvalue_6))
  (bind _returnvalue_7 (* _worlddirection 2e+01))
  (bind _returnvalue_8 (+ _returnvalue _returnvalue_7))
  (Utilities|FlowControl|DoOnce false
    (:Completed
      (bind _alpha (Timeline|TransitionLocation Play)
        (:Update
          (Transformation|SetActorLocation (Math|Vector|Lerp(Vector) _returnvalue (Math|Vector|MakeVector (.x _returnvalue_8) (.y _returnvalue_8) (.Z (Math|Vector|BreakVector _returnvalue))) _alpha) false false))
        (:Finished
          (Development|PrintString "Hello"))))))

(fn ConstructionScript
  (bind _outrownames (DataTable|GetDataTableRowNames "/Game/Blueprints/Plants/DT_Plantes.DT_Plantes"))
  (Variables|Default|SetOut%20Row%20Names _outrownames))